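; BP_FlamePillar is a flame pillar actor whose fire light flickers.
; On BeginPlay it randomly starts one of two intensity timelines, either forward or in reverse, varying the initial flicker between instances.
; Each timeline update sets FireLight intensity to the curve value times BaseIntensity.
; When one timeline finishes it plays the other from the start, so the flicker loops without Tick.
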(event `self.ReceiveBeginPlay`
  (switch `int` (`KismetMathLibrary.RandomIntegerInRange` 0 3)
    (:`0`
      (bind (_direction _intensity) (`Timeline|FlameIntensity` :!via `PlayFromStart` :!label _label)
        (:`Update`
          (`LightComponent.SetIntensity` (`self.FireLight`) (* _intensity (`self.BaseIntensity`))))
        (:`Finished`
          (bind (_direction_2 _intensity_2) (`Timeline|FlameIntensity2` :!via `PlayFromStart` :!label _label_2)
            (:`Update`
              (`LightComponent.SetIntensity` (`self.FireLight`) (* _intensity_2 (`self.BaseIntensity`))))
            (:`Finished`
              (goto _label :!via `PlayFromStart`))))))
    (:`1`
      (goto _label :!via `ReverseFromEnd`))
    (:`2`
      (goto _label_2 :!via `PlayFromStart`))
    (:`3`
      (goto _label_2 :!via `ReverseFromEnd`))))

(fn `UserConstructionScript`)