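; Player gameplay ability that casts a fire bolt toward the point under the mouse.
; It turns the player to face that target, then plays the montage from the player's ranged attack info tagged for FireBolt.
; The montage's gameplay event spawns the fire bolt projectile, carrying its damage effect, from the attack's combat socket.
; The ability ends shortly after spawning, or when the montage completes, is interrupted or cancelled.
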(event `self.K2_ActivateAbility`
  (bind (_asynctaskproxy _datahandle) (`TargetDataUnderMouse.GetTargetDataUnderMouse`)
    (:`ValidData`
      (bind _asbp_player (cast `/Game/Blueprints/Character/Player/BP_Player` (`self.GetAvatarActorFromActorInfo`)))
      (bind (_bblockinghit _binitialoverlap _time _distance _location) (`GameplayStatics.BreakHitResult` (`AbilitySystemBlueprintLibrary.GetHitResultFromTargetData` _datahandle)))
      (`CombatInterface.SetFacingTargetLocation` _asbp_player _location)
      (for _array_element (`CharacterBase.RangedAttackInfos` _asbp_player)
        (bind (_montage _attacktag _attacksocketname) (break `RangedAttackInfo` _array_element))
        (if (== _attacktag (struct :`TagName` "Event.Montage.FireBolt"))
          (break)))
      (`AbilityTask_PlayMontageAndWait.CreatePlayMontageAndWaitProxy` "None" _montage
        (:`then`
          (`AbilityTask_WaitGameplayEvent.WaitGameplayEvent` _attacktag null
            (:`EventReceived`
              (bind _returnvalue (`CombatInterface.GetCombatSocketLocation` _asbp_player _attacksocketname))
              (`self.SpawnProjectile` _location _returnvalue (make `ProjectileInfo` "/Game/Blueprints/AbilitySystem/GameplayAbilities/Player/FireBolt/BP_FireBolt.BP_FireBolt_C" "/Game/Blueprints/AbilitySystem/GameplayAbilities/Player/FireBolt/GE_FireBolt.GE_FireBolt_C"))
              (`KismetSystemLibrary.Delay` 0.2)
              (`self.K2_EndAbility`))))
        (:`OnCompleted`
          (`self.K2_EndAbility` :!label _label))
        (:`OnInterrupted`
          (goto _label))
        (:`OnCancelled`
          (goto _label))))))