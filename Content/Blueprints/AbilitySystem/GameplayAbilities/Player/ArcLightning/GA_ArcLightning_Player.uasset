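; Player gameplay ability for a channeled arc lightning beam at the target under the mouse.
; A cast montage event disables movement and traces from the weapon tip to place a beam cue.
; On a character hit, beams chain to nearby enemies, limited by ability level, and a looping timer pays cost to damage and debuff them all.
; Input release ends the channel, committing cooldown if it fired; ending removes the beam cues.
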(event `self.K2_ActivateAbility`
  (bind _mousehitlocation (`self.MouseHitLocation`))
  (bind _mousehitactor (`self.MouseHitActor`))
  (set `self.bBeamed` false)
  (bind (_asynctaskproxy _datahandle) (`TargetDataUnderMouse.GetTargetDataUnderMouse`)
    (:`ValidData`
      (`self.StoreMouseDataInfo` (`AbilitySystemBlueprintLibrary.GetHitResultFromTargetData` _datahandle))
      (`self.StoreOwnerPlayerController`)
      (bind _asbp_player (cast `/Game/Blueprints/Character/Player/BP_Player` (`self.GetAvatarActorFromActorInfo`)))
      (message `CombatInterface.SetFacingTargetLocation` _asbp_player (`self.MouseHitLocation`))
      (`AbilityTask_PlayMontageAndWait.CreatePlayMontageAndWaitProxy` "None" "/Game/Assets/Characters/Aura/Animations/Abilities/AM_Cast_Shock.AM_Cast_Shock"
        (:`then`
          (`AbilityTask_WaitGameplayEvent.WaitGameplayEvent` (struct :`TagName` "Event.Montage.Electrocute") null true
            (:`then`
              (`AbilityTask_WaitInputRelease.WaitInputRelease` false
                (:`OnRelease`
                  (`KismetSystemLibrary.K2_ClearAndInvalidateTimerHandle` (`self.TimerHandle`))
                  (if (`self.bBeamed`)
                    (set `/Game/Blueprints/Character/Player/BP_Player.bInShockLoop` false _asbp_player)
                    (set `PlayerController.bShowMouseCursor` true (`self.OwnerPlayerController`))
                    (bind _charactermovement (`Character.CharacterMovement` _asbp_player))
                    (`CharacterMovementComponent.SetMovementMode` _charactermovement "MOVE_Walking" 0)
                    (`self.K2_CommitAbilityCooldown` false)
                    (`self.K2_EndAbility`)
                    (else
                      (`self.K2_EndAbility`))))))
            (:`EventReceived`
              (set `self.bBeamed` true)
              (set `/Game/Blueprints/Character/Player/BP_Player.bInShockLoop` true _asbp_player)
              (`self.K2_ExecuteGameplayCueWithParams` (struct :`TagName` "GameplayCue.AttackEffect.Sound") (`AbilitySystemBlueprintLibrary.MakeGameplayCueParameters` 0.0 0.0 (struct) (struct) (struct) (struct) (struct) (`Actor.K2_GetActorLocation` (`self.GetAvatarActorFromActorInfo`)) (0.0 0.0 0.0) null null "/Game/Assets/Sounds/Abilities/Shock/sfx_Shock.sfx_Shock"))
              (set `PlayerController.bShowMouseCursor` false (`self.OwnerPlayerController`))
              (`CharacterMovementComponent.DisableMovement` _charactermovement)
              (bind _weapon (`CharacterBase.Weapon` _asbp_player))
              (bind _outhit (`KismetSystemLibrary.SphereTraceSingle` (`SceneComponent.GetSocketLocation` _weapon "TipSocket") _mousehitlocation 10.0 "TraceTypeQuery1" false (`|MakeArray` (`self.GetAvatarActorFromActorInfo`)) "ForDuration"))
              (bind (_bblockinghit _binitialoverlap _time _distance _location _impactpoint _normal _impactnormal _physmat _hitactor) (`GameplayStatics.BreakHitResult` _outhit))
              (if _bblockinghit
                (set `self.MouseHitLocation` _impactpoint)
                (set `self.MouseHitActor` _hitactor))
              (`GameplayCueFunctionLibrary.AddGameplayCueOnActor` _asbp_player (struct :`TagName` "GameplayCue.AttackEffect.Beam") (`AbilitySystemBlueprintLibrary.MakeGameplayCueParameters` 0.0 0.0 (struct) (struct) (struct) (struct) (struct) _mousehitlocation (0.0 0.0 0.0) null null "/Game/Assets/Effects/Shock/NS_ElectricBeam.NS_ElectricBeam" null 1 1 _weapon))
              (cast `CharacterBase` _mousehitactor)
              (bind _outactors (`KismetSystemLibrary.SphereOverlapActors` (`Actor.K2_GetActorLocation` _mousehitactor) 200.0 (`|MakeArray` "ObjectTypeQuery3" :!type "EObjectTypeQuery Enum") "/Game/Blueprints/Character/Enemy/BP_Enemy.BP_Enemy_C" (`|MakeArray` _mousehitactor)))
              (for (_array_element _array_index) _outactors
                (if (> _array_index (/ (`self.GetAbilityLevel`) 2))
                  (break)
                  (else
                    (bind _returnvalue (`AbilitySystemBlueprintLibrary.MakeGameplayCueParameters` 0.0 0.0 (struct) (struct) (struct) (struct) (struct) (`Actor.K2_GetActorLocation` _array_element) (0.0 0.0 0.0) null null null null 1 1 (`Actor.RootComponent` (`self.MouseHitActor`))))
                    (`GameplayCueFunctionLibrary.AddGameplayCueOnActor` _array_element (struct :`TagName` "GameplayCue.AttackEffect.Beam") _returnvalue)
                    (`BlueprintMapLibrary.Map_Add` (`self.HitActorsMap`) _array_element _returnvalue)
                    (`KismetArrayLibrary.Array_Add` (`self.HitActors`) _array_element))))
              (bind _returnvalue_2 (`KismetSystemLibrary.K2_SetTimerDelegate` (delegate `ApplyEffect`) (`self.DamageDeltaTime`) true))
              (set `self.TimerHandle` _returnvalue_2))))))))

(event `ApplyEffect`
  (bind _returnvalue (`self.K2_CommitAbilityCost` false))
  (if _returnvalue
    (`self.ApplyDamageAndDebuff` "/Game/Blueprints/AbilitySystem/GameplayAbilities/Player/ArcLightning/GE_ArcLightning.GE_ArcLightning_C")))

(event `self.K2_OnEndAbility`
  (params (bWasCancelled :type Boolean))
  (bind _hitactorsmap (`self.HitActorsMap`))
  (bind _hitactors (`self.HitActors`))
  (`self.K2_RemoveGameplayCue` (struct :`TagName` "GameplayCue.AttackEffect.Beam"))
  (for _array_element _hitactors
    (`GameplayCueFunctionLibrary.RemoveGameplayCueOnActor` _array_element (struct :`TagName` "GameplayCue.AttackEffect.Beam") (`BlueprintMapLibrary.Map_Find` _hitactorsmap _array_element)))
  (`KismetArrayLibrary.Array_Clear` _hitactors)
  (`BlueprintMapLibrary.Map_Clear` _hitactorsmap))

(fn `ApplyDamageAndDebuff`
  (params (DamageEffectClass :type "GameplayEffect Class Reference"))
  (bind _returnvalue (`self.GetAbilitySystemComponentFromActorInfo`))
  (bind _returnvalue_2 (`AbilitySystemComponent.MakeOutgoingSpec` _returnvalue DamageEffectClass (`KismetMathLibrary.Conv_IntToDouble` (`self.GetAbilityLevel`)) (`AbilitySystemComponent.MakeEffectContext` _returnvalue)))
  (bind _ascharacter_base (cast `CharacterBase` (`self.MouseHitActor`)))
  (bind _returnvalue_3 (`AbilitySystemBlueprintLibrary.GetAbilitySystemComponent` _ascharacter_base))
  (`AbilitySystemComponent.BP_ApplyGameplayEffectSpecToTarget` _returnvalue _returnvalue_2 _returnvalue_3)
  (`self.ApplyDebuff` _returnvalue_3)
  (for _array_element (`self.HitActors`)
    (bind _ascharacter_base_2 (cast `CharacterBase` _array_element))
    (bind _returnvalue_4 (`AbilitySystemBlueprintLibrary.GetAbilitySystemComponent` _ascharacter_base_2))
    (`AbilitySystemComponent.BP_ApplyGameplayEffectSpecToTarget` _returnvalue _returnvalue_2 _returnvalue_4)
    (`self.ApplyDebuff` _returnvalue_4)))