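; Enemy melee Gameplay Ability that faces the combat target, plays a random attack montage and damages characters in the swing path.
; Montage gameplay events mark swing start and end, sampling the weapon socket at each for one sphere trace between them.
; Each unique living character hit receives GE_EnemyAttack and a blood Niagara cue, with one impact sound cue if anything was hit.
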(event `self.K2_ActivateAbility`
  (bind _returnvalue (`self.GetAvatarActorFromActorInfo`))
  (bind _hitactorset (`self.HitActorSet`))
  (bind _asbp_enemy (cast `/Game/Blueprints/Character/Enemy/BP_Enemy` _returnvalue))
  (`CombatInterface.SetFacingTargetLocation` _asbp_enemy (`Actor.K2_GetActorLocation` (`Enemy.CombatTarget` _asbp_enemy)))
  (bind _output_get (set `self.AttackInfo` (`KismetArrayLibrary.Array_Random` (`CharacterBase.AttackInfos` _asbp_enemy))))
  (bind (_montage _attackstarttag _attackendtag _attacksocketname _attackradius _impactsound) (break `AttackInfo` _output_get))
  (`AbilityTask_PlayMontageAndWait.CreatePlayMontageAndWaitProxy` "None" _montage
    (:`then`
      (`AbilityTask_WaitGameplayEvent.WaitGameplayEvent` _attackstarttag null
        (:`EventReceived`
          (bind _returnvalue_2 (message `CombatInterface.GetCombatSocketLocation` _returnvalue _attacksocketname))
          (`AbilityTask_WaitGameplayEvent.WaitGameplayEvent` _attackendtag null
            (:`EventReceived`
              (bind _returnvalue_3 (message `CombatInterface.GetCombatSocketLocation` _returnvalue _attacksocketname))
              (bind _outhits (`KismetSystemLibrary.SphereTraceMultiForObjects` :`Start` _returnvalue_2 :`End` _returnvalue_3 :`Radius` _attackradius :`ObjectTypes` (`|MakeArray` "ObjectTypeQuery3" :!type "EObjectTypeQuery Enum") :`DrawDebugType` "ForDuration"))
              (`BlueprintSetLibrary.Set_Clear` (`self.HitActorSet`))
              (set `self.bHitTarget` false)
              (for _array_element _outhits
                (bind (_bblockinghit _binitialoverlap _time _distance _location _impactpoint _normal _impactnormal _physmat _hitactor) (`GameplayStatics.BreakHitResult` _array_element))
                (if (not (`BlueprintSetLibrary.Set_Contains` _hitactorset _hitactor))
                  (bind _ascharacter_base (cast `CharacterBase` _hitactor))
                  (if (not (`CombatInterface.IsDead` _ascharacter_base))
                    (bind _asbp_enemy_2 (cast `/Game/Blueprints/Character/Enemy/BP_Enemy` (`self.GetAvatarActorFromActorInfo`)))
                    (`BlueprintSetLibrary.Set_Add` _hitactorset _hitactor)
                    (bind _returnvalue_4 (`AbilitySystemBlueprintLibrary.GetAbilitySystemComponent` _asbp_enemy_2))
                    (`AbilitySystemComponent.BP_ApplyGameplayEffectToTarget` _returnvalue_4 "/Game/Blueprints/AbilitySystem/GameplayAbilities/Enemy/GE_EnemyAttack.GE_EnemyAttack_C" (`AbilitySystemBlueprintLibrary.GetAbilitySystemComponent` _ascharacter_base) 1.0 (`AbilitySystemComponent.MakeEffectContext` _returnvalue_4))
                    (set `self.bHitTarget` true)
                    (`self.K2_ExecuteGameplayCueWithParams` (struct :`TagName` "GameplayCue.AttackEffect.Niagara") (`AbilitySystemBlueprintLibrary.MakeGameplayCueParameters` 0.0 0.0 (struct) (struct) (struct) (struct) (struct) _location (0.0 0.0 0.0) null null (`CharacterBase.BloodEffect` _ascharacter_base))))))
              (if (`self.bHitTarget`)
                (`self.K2_ExecuteGameplayCueWithParams` (struct :`TagName` "GameplayCue.AttackEffect.Sound") (`AbilitySystemBlueprintLibrary.MakeGameplayCueParameters` 0.0 0.0 (struct) (struct) (struct) (struct) (struct) _returnvalue_2 (0.0 0.0 0.0) null null _impactsound)))
              (`self.K2_EndAbility`))))))
    (:`OnCompleted`
      (`self.K2_EndAbility` :!label _label))
    (:`OnInterrupted`
      (goto _label))
    (:`OnCancelled`
      (goto _label))))