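; Gameplay ability that makes the demon enemy throw a projectile at its combat target.
; It turns the demon toward the target and plays a montage picked at random from its ranged attack infos.
; When that attack's tagged gameplay event arrives, it spawns a random projectile from the attack's socket, aimed at the target's current location, then ends without stopping the montage.
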(event `self.K2_ActivateAbility`
  (bind _asbp_demon (cast `/Game/Blueprints/Character/Enemy/Demon/BP_Demon` (`self.GetAvatarActorFromActorInfo`)))
  (bind _returnvalue (`Actor.K2_GetActorLocation` (`Enemy.CombatTarget` _asbp_demon)))
  (`CombatInterface.SetFacingTargetLocation` _asbp_demon _returnvalue)
  (bind _output_get (set `self.AttackInfo` (`KismetArrayLibrary.Array_Random` (`CharacterBase.RangedAttackInfos` _asbp_demon))))
  (bind (_montage _attacktag _attacksocketname) (break `RangedAttackInfo` _output_get))
  (`AbilityTask_PlayMontageAndWait.CreatePlayMontageAndWaitProxy` "None" _montage 1.0 "None" false
    (:`then`
      (`AbilityTask_WaitGameplayEvent.WaitGameplayEvent` _attacktag null
        (:`EventReceived`
          (bind _returnvalue_2 (message `CombatInterface.GetCombatSocketLocation` _asbp_demon _attacksocketname))
          (bind _output_get_2 (set `self.ProjectileInfo` (`KismetArrayLibrary.Array_Random` (`/Game/Blueprints/Character/Enemy/Demon/BP_Demon.ProjectileInfos` _asbp_demon))))
          (`self.SpawnProjectile` _returnvalue _returnvalue_2 _output_get_2)
          (`self.K2_EndAbility`))))
    (:`OnCompleted`
      (`self.K2_EndAbility` :!label _label))
    (:`OnInterrupted`
      (goto _label))
    (:`OnCancelled`
      (goto _label))))