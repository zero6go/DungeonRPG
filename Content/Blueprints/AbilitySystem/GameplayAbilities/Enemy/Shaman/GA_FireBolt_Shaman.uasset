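; Fire bolt gameplay ability for the Shaman enemy, which attacks its combat target at range.
; On activation it turns the enemy toward the target and plays a random montage from its ranged attack infos.
; The attack's gameplay event tag triggers spawning a BP_FireBolt projectile with GE_FireBolt damage from that attack's socket toward the target.
; The ability ends after the spawn, or when the montage completes, is interrupted or is cancelled.
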(event `self.K2_ActivateAbility`
  (bind _asbp_enemy (cast `/Game/Blueprints/Character/Enemy/BP_Enemy` (`self.GetAvatarActorFromActorInfo`)))
  (bind _returnvalue (`Actor.K2_GetActorLocation` (`Enemy.CombatTarget` _asbp_enemy)))
  (`CombatInterface.SetFacingTargetLocation` _asbp_enemy _returnvalue)
  (bind _output_get (set `self.AttackInfo` (`KismetArrayLibrary.Array_Random` (`CharacterBase.RangedAttackInfos` _asbp_enemy))))
  (bind (_montage _attacktag _attacksocketname) (break `RangedAttackInfo` _output_get))
  (`AbilityTask_PlayMontageAndWait.CreatePlayMontageAndWaitProxy` "None" _montage 1.0 "None" false
    (:`then`
      (`AbilityTask_WaitGameplayEvent.WaitGameplayEvent` _attacktag null
        (:`EventReceived`
          (bind _returnvalue_2 (message `CombatInterface.GetCombatSocketLocation` _asbp_enemy _attacksocketname))
          (`self.SpawnProjectile` _returnvalue _returnvalue_2 (make `ProjectileInfo` "/Game/Blueprints/AbilitySystem/GameplayAbilities/Player/FireBolt/BP_FireBolt.BP_FireBolt_C" "/Game/Blueprints/AbilitySystem/GameplayAbilities/Player/FireBolt/GE_FireBolt.GE_FireBolt_C"))
          (`self.K2_EndAbility`))))
    (:`OnCompleted`
      (`self.K2_EndAbility` :!label _label))
    (:`OnInterrupted`
      (goto _label))
    (:`OnCancelled`
      (goto _label))))