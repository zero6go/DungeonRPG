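; Shaman enemy gameplay ability that summons a random minion during a summon montage.
; It picks the spawn location on activation, plays the montage at reduced rate and waits for the summon montage event.
; On that event it spawns a minion no higher in level than the Shaman, increments MinionCount and fires a Niagara gameplay cue just below the spawn point.
; The ability ends after summoning or when the montage completes, is interrupted or is cancelled.
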(event `self.K2_ActivateAbility`
  (bind _returnvalue (`self.GetSpawnLocation`))
  (bind _asbp_enemy (cast `/Game/Blueprints/Character/Enemy/BP_Enemy` (`self.GetAvatarActorFromActorInfo`)))
  (`AbilityTask_PlayMontageAndWait.CreatePlayMontageAndWaitProxy` "None" "/Game/Assets/Enemies/Shaman/Animations/AM_Shaman_Summon.AM_Shaman_Summon" 0.5
    (:`then`
      (`AbilityTask_WaitGameplayEvent.WaitGameplayEvent` (struct :`TagName` "Event.Montage.Summon") null
        (:`EventReceived`
          (`self.SpawnMinion` (`self.GetRandomMinionClass`) _returnvalue (`KismetMathLibrary.RandomIntegerInRange` 1 (`CharacterBase.GetCharacterLevel` _asbp_enemy)))
          (`/Engine/EditorBlueprintResources/StandardMacros.IncrementInt` (`CharacterBase.MinionCount` _asbp_enemy)
            (:`  `
              (`self.K2_ExecuteGameplayCueWithParams` (struct :`TagName` "GameplayCue.AttackEffect.Niagara") (`AbilitySystemBlueprintLibrary.MakeGameplayCueParameters` 0.0 0.0 (struct) (struct) (struct) (struct) (struct) (`KismetMathLibrary.MakeVector` (.x _returnvalue) (.y _returnvalue) (- (.z _returnvalue) 50.0)) (0.0 0.0 0.0) null null (`self.SummonEffect`)))
              (`self.K2_EndAbility`))))))
    (:`OnCompleted`
      (`self.K2_EndAbility` :!label _label))
    (:`OnInterrupted`
      (goto _label))
    (:`OnCancelled`
      (goto _label))))

(event `SpawnSound`)